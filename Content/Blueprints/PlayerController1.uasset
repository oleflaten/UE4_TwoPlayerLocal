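; Player 1's controller, which also sets up and drives a second player character.
; On BeginPlay it spawns PlayerController2 and ThirdPersonCharacter2 at a hardcoded location, then has the new controller possess that character.
; It receives both players' move axes itself, applying one set to its own pawn and the other to Character2.
; Each character moves relative to its own controller's rotation.
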(event EventBeginPlay
  (bind _returnvalue (Math|Transform|MakeTransform "-900.000000,900.000000,230.000000"))
  ;[1 1 1] Setup other player
  (Development|PrintString "Hello")
  (bind _returnvalue_2 (Game|SpawnActorfromClass "/Game/Blueprints/PlayerController2.PlayerController2_C" _returnvalue "Undefined" 0 0))
  (Variables|Default|SetController2 _returnvalue_2)
  (bind _returnvalue_3 (Game|SpawnActorfromClass "/Game/ThirdPersonCPP/Blueprints/ThirdPersonCharacter2.ThirdPersonCharacter2_C" _returnvalue "Undefined" 0 0))
  (bind _output_get (Variables|Default|SetCharacter2 _returnvalue_3))
  (Pawn|Possess (Variables|Default|GetController2) _output_get))

(event Input|AxisEvents|InputAxisMoveForward1
  (params (AxisValue :type Float%20%28single-precision%29))
  (bind _returnvalue (Pawn|GetControlledPawn))
  ;[1 1 1] Movent for Player 1
  (Pawn|Input|AddMovementInput _returnvalue (Math|Vector|GetForwardVector (Pawn|GetControlRotation (Pawn|GetController _returnvalue) :!class /Script/Engine.Controller)) AxisValue false))

(event Input|AxisEvents|InputAxisMoveForward2
  (params (AxisValue :type Float%20%28single-precision%29))
  (bind _character2 (Variables|Default|GetCharacter2))
  ;[1 1 1] Movement for Player 2
  (Pawn|Input|AddMovementInput _character2 (Math|Vector|GetForwardVector (Pawn|GetControlRotation (Pawn|GetController _character2) :!class /Script/Engine.Controller)) AxisValue false))

(event Input|AxisEvents|InputAxisMoveRight2
  (params (AxisValue :type Float%20%28single-precision%29))
  (bind _character2 (Variables|Default|GetCharacter2))
  ;[1 1 1] Movement for Player 2
  (Pawn|Input|AddMovementInput _character2 (Math|Vector|GetRightVector (Pawn|GetControlRotation (Pawn|GetController _character2) :!class /Script/Engine.Controller)) AxisValue false))

(event Input|AxisEvents|InputAxisMoveRight1
  (params (AxisValue :type Float%20%28single-precision%29))
  (bind _returnvalue (Pawn|GetControlledPawn))
  ;[1 1 1] Movent for Player 1
  (Pawn|Input|AddMovementInput _returnvalue (Math|Vector|GetRightVector (Pawn|GetControlRotation (Pawn|GetController _returnvalue) :!class /Script/Engine.Controller)) AxisValue false))

(fn ConstructionScript)